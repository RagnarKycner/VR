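; Map chunk actor with a dynamic mesh that can have holes dug into it at runtime.
; The construction script copies the Mesh static mesh into the DynamicMeshComponent, applies PN tessellation and enables complex-as-simple collision.
; DigHole uses Geometry Script to boolean-subtract a pooled cylinder at the given location, converted to local space with the component's scale compensated.
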(fn `DigHole`
  (params (Location :type "Vector Structure"))
  (bind _dynamicmeshcomponent (`self.DynamicMeshComponent`))
  (bind (_returnvalue_location _returnvalue_rotation _returnvalue_scale) (`KismetMathLibrary.BreakTransform` (`SceneComponent.K2_GetComponentToWorld` _dynamicmeshcomponent)))
  (bind _returnvalue (`self.AllocateComputeMesh`))
  (bind _returnvalue_2 (`GeometryScriptLibrary_MeshPrimitiveFunctions.AppendCylinder` _returnvalue (struct) (`KismetMathLibrary.MakeTransform` (`KismetMathLibrary.InverseTransformLocation` (`SceneComponent.K2_GetComponentToWorld` _dynamicmeshcomponent) Location) (struct) (/ (1.0 1.0 1.0) _returnvalue_scale)) 33.0 100.0 12 0 true "Center" null))
  (bind _returnvalue_3 (`BaseDynamicMeshComponent.GetDynamicMesh` (`self.DynamicMeshComponent`)))
  (`GeometryScriptLibrary_MeshBooleanFunctions.ApplyMeshBoolean` _returnvalue_3 (`KismetMathLibrary.MakeTransform` (0.0 0.0 0.0)) _returnvalue_2 (struct) "Subtract" (struct) null)
  (`self.ReleaseAllComputeMeshes`))

(fn `UserConstructionScript`
  (bind _returnvalue (`BaseDynamicMeshComponent.GetDynamicMesh` (`self.DynamicMeshComponent`)))
  (bind _output_get (set `self.DynamicMesh` _returnvalue))
  (bind _returnvalue_2 (`DynamicMesh.Reset` _output_get))
  (bind _returnvalue_3 (`GeometryScriptLibrary_StaticMeshFunctions.CopyMeshFromStaticMesh` (`StaticMeshComponent.StaticMesh` (`self.mesh`)) _returnvalue_2 (struct) (struct) null)
    (:`Success`
      (`GeometryScriptLibrary_MeshSubdivideFunctions.ApplyPNTessellation` _returnvalue_3 (struct) 2 null)
      (`DynamicMeshComponent.SetComplexAsSimpleCollisionEnabled` (`self.DynamicMeshComponent`) true true))))