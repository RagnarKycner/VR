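; BP_Tree is a tree actor that selects its set of three tree states to match the game's current tree ID.
; On BeginPlay it finds BP_Game and compares its TreeID against a fixed list through nested branches.
; The match fills the TreeStates map: ID 6 uses the Tree1 variants, other listed IDs use Tree2, with ID 8 in reverse order.
; This graph only builds the map and never applies it.
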(event `self.ReceiveBeginPlay`
  (bind _returnvalue (`GameplayStatics.GetActorOfClass` "/Game/zVRContent/blueprints/BP_Game.BP_Game_C"))
  (bind _output_get (set `self.BP_Game` _returnvalue))
  (bind _treeid (`/Game/zVRContent/blueprints/BP_Game.TreeID` _output_get))
  (if (== 6 _treeid)
    (set `self.TreeStates` (`|MakeMap` 1 "/Game/zVRContent/Meshes/trees/tree1_1.tree1_1" 2 "/Game/zVRContent/Meshes/trees/tree1_2.tree1_2" 3 "/Game/zVRContent/Meshes/trees/tree1_3.tree1_3" :!valuetype "StaticMesh Object Reference"))
    (elif (== 8 _treeid)
      (set `self.TreeStates` (`|MakeMap` 1 "/Game/zVRContent/Meshes/trees/tree2_3.tree2_3" 2 "/Game/zVRContent/Meshes/trees/tree2_2.tree2_2" 3 "/Game/zVRContent/Meshes/trees/tree2_1.tree2_1" :!valuetype "StaticMesh Object Reference"))
      (elif (== 10 _treeid)
        (set `self.TreeStates` (`|MakeMap` 1 "/Game/zVRContent/Meshes/trees/tree2_1.tree2_1" 2 "/Game/zVRContent/Meshes/trees/tree2_2.tree2_2" 3 "/Game/zVRContent/Meshes/trees/tree2_3.tree2_3" :!valuetype "StaticMesh Object Reference"))
        (elif (== 12 _treeid)
          (set `self.TreeStates` (`|MakeMap` 1 "/Game/zVRContent/Meshes/trees/tree2_1.tree2_1" 2 "/Game/zVRContent/Meshes/trees/tree2_2.tree2_2" 3 "/Game/zVRContent/Meshes/trees/tree2_3.tree2_3" :!valuetype "StaticMesh Object Reference"))
          (elif (== 15 _treeid)
            (set `self.TreeStates` (`|MakeMap` 1 "/Game/zVRContent/Meshes/trees/tree2_1.tree2_1" 2 "/Game/zVRContent/Meshes/trees/tree2_2.tree2_2" 3 "/Game/zVRContent/Meshes/trees/tree2_3.tree2_3" :!valuetype "StaticMesh Object Reference"))
            (elif (== 20 _treeid)
              (set `self.TreeStates` (`|MakeMap` 1 "/Game/zVRContent/Meshes/trees/tree2_1.tree2_1" 2 "/Game/zVRContent/Meshes/trees/tree2_2.tree2_2" 3 "/Game/zVRContent/Meshes/trees/tree2_3.tree2_3" :!valuetype "StaticMesh Object Reference"))
              (elif (== 24 _treeid)
                (set `self.TreeStates` (`|MakeMap` 1 "/Game/zVRContent/Meshes/trees/tree2_1.tree2_1" 2 "/Game/zVRContent/Meshes/trees/tree2_2.tree2_2" 3 "/Game/zVRContent/Meshes/trees/tree2_3.tree2_3" :!valuetype "StaticMesh Object Reference"))
                (elif (== 30 _treeid)
                  (set `self.TreeStates` (`|MakeMap` 1 "/Game/zVRContent/Meshes/trees/tree2_1.tree2_1" 2 "/Game/zVRContent/Meshes/trees/tree2_2.tree2_2" 3 "/Game/zVRContent/Meshes/trees/tree2_3.tree2_3" :!valuetype "StaticMesh Object Reference"))
                  (elif (== 40 _treeid)
                    (set `self.TreeStates` (`|MakeMap` 1 "/Game/zVRContent/Meshes/trees/tree2_1.tree2_1" 2 "/Game/zVRContent/Meshes/trees/tree2_2.tree2_2" 3 "/Game/zVRContent/Meshes/trees/tree2_3.tree2_3" :!valuetype "StaticMesh Object Reference"))
                    (elif (== 60 _treeid)
                      (set `self.TreeStates` (`|MakeMap` 1 "/Game/zVRContent/Meshes/trees/tree2_1.tree2_1" 2 "/Game/zVRContent/Meshes/trees/tree2_2.tree2_2" 3 "/Game/zVRContent/Meshes/trees/tree2_3.tree2_3" :!valuetype "StaticMesh Object Reference")))))))))))))

(fn `UserConstructionScript`)