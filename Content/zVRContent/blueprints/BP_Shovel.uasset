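; BP_Shovel is a VR shovel that digs holes in map chunks when the player holds it.
; When its box overlaps a BP_MapChunk while either hand holds a shovel, it traces along the plane's up vector to find the chunk surface.
; On a hit it calls the chunk's DigHole and records the location on the player.
; A DiggedHole flag blocks further digs until the box leaves a chunk.
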(event `self.Box.OnComponentBeginOverlap`
  (params (OverlappedComponent :type "PrimitiveComponent Object Reference") (OtherActor :type "Actor Object Reference") (OtherComp :type "PrimitiveComponent Object Reference") (OtherBodyIndex :type Integer) (bFromSweep :type Boolean) (SweepResult :type "HitResult Structure (by ref)"))
  (bind _plane (`self.Plane`))
  (bind _returnvalue (`SceneComponent.K2_GetComponentLocation` _plane))
  (bind _heldcomponentleft (`/Game/VRTemplate/Blueprints/VRPawn.HeldComponentLeft` (`/Game/zVRContent/blueprints/BP_Game.PlayerRef` (`self.GameRef`))))
  (bind _heldcomponentright (`/Game/VRTemplate/Blueprints/VRPawn.HeldComponentRight` (`/Game/zVRContent/blueprints/BP_Game.PlayerRef` (`self.GameRef`))))
  (if (`self.DiggedHole`)
    _
    (elif (`KismetMathLibrary.ClassIsChildOf` (`GameplayStatics.GetObjectClass` (`ActorComponent.GetOwner` OtherComp)) "/Game/zVRContent/blueprints/BP_MapChunk.BP_MapChunk_C")
      (`|ExecutionSequence`
        (:`then_0`
          (if (`KismetSystemLibrary.IsValid` _heldcomponentleft)
            (if (`KismetMathLibrary.ClassIsChildOf` (`GameplayStatics.GetObjectClass` (`ActorComponent.GetOwner` _heldcomponentleft)) "BP_Shovel_C")
              (bind _outactors (`GameplayStatics.GetAllActorsWithTag` "tag" :!label _label))
              (`KismetArrayLibrary.Array_Add` _outactors self)
              (bind (_outhit _returnvalue_2) (`KismetSystemLibrary.LineTraceSingle` _returnvalue (+ _returnvalue (* (`SceneComponent.GetUpVector` _plane) 500.0)) "TraceTypeQuery1" false _outactors))
              (if _returnvalue_2
                (bind (_bblockinghit _binitialoverlap _time _distance _location _impactpoint _normal _impactnormal _physmat _hitactor) (`GameplayStatics.BreakHitResult` _outhit))
                (if (`KismetMathLibrary.ClassIsChildOf` (`GameplayStatics.GetObjectClass` _hitactor) "/Game/zVRContent/blueprints/BP_MapChunk.BP_MapChunk_C")
                  (bind _asbp_map_chunk (cast `/Game/zVRContent/blueprints/BP_MapChunk` _hitactor))
                  (`/Game/zVRContent/blueprints/BP_MapChunk.DigHole` _asbp_map_chunk _location)
                  (`KismetArrayLibrary.Array_Add` (`/Game/VRTemplate/Blueprints/VRPawn.HoleLocation` (`/Game/zVRContent/blueprints/BP_Game.PlayerRef` (`self.GameRef`))) _location)
                  (set `self.DiggedHole` true))))))
        (:`then_1`
          (if (`KismetSystemLibrary.IsValid` _heldcomponentright)
            (if (`KismetMathLibrary.ClassIsChildOf` (`GameplayStatics.GetObjectClass` (`ActorComponent.GetOwner` _heldcomponentright)) "BP_Shovel_C")
              (goto _label))))))))

(event `self.Box.OnComponentEndOverlap`
  (params (OverlappedComponent :type "PrimitiveComponent Object Reference") (OtherActor :type "Actor Object Reference") (OtherComp :type "PrimitiveComponent Object Reference") (OtherBodyIndex :type Integer))
  (if (`KismetMathLibrary.ClassIsChildOf` (`GameplayStatics.GetObjectClass` (`ActorComponent.GetOwner` OtherComp)) "/Game/zVRContent/blueprints/BP_MapChunk.BP_MapChunk_C")
    (set `self.DiggedHole` false)))

(event `self.ReceiveBeginPlay`
  (bind _returnvalue (`GameplayStatics.GetActorOfClass` "/Game/zVRContent/blueprints/BP_Game.BP_Game_C"))
  (set `self.GameRef` _returnvalue))

(fn `UserConstructionScript`)