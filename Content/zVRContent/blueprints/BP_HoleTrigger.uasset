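; BP_HoleTrigger is a hole trigger actor that turns into a tree when a sapling is placed in it.
; When the actor stored in its Sapling variable overlaps it, it spawns BP_Tree at its own transform and destroys itself, leaving the sapling untouched.
; It caches the first BP_Game on BeginPlay, but the only use of that reference, resetting TreeID, is disconnected.
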(event `self.ReceiveBeginPlay`
  (bind _outactors (`GameplayStatics.GetAllActorsOfClass` "/Game/zVRContent/blueprints/BP_Game.BP_Game_C"))
  (set `self.BP_Game` (`|GetArrayItem` _outactors)))

(event `self.ReceiveActorBeginOverlap`
  (params (OtherActor :type "Actor Object Reference"))
  (if (== OtherActor "/Game/zVRContent/blueprints/Sapling.Sapling")
    (`|SpawnActorFromClass` "/Game/zVRContent/blueprints/BP_Tree.BP_Tree_C" (`self.GetTransform` self) "AlwaysSpawn" "MultiplyWithRoot" null null)
    (`self.K2_DestroyActor`)))

(fn `UserConstructionScript`)