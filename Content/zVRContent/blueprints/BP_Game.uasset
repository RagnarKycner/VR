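; BP_Game manages world state for the VR game: map chunk terrain, tree growth and player oxygen.
; BeginPlay copies chunk meshes into tessellated, collidable dynamic meshes, registers one tree's oxygen zone and adds a radial-blur post-process to the pawn camera.
; A P-key action runs WorldManaging, restoring chunk holes from cached static meshes and advancing queued tree stages.
; Tick checks oxygen-zone overlap, but the oxygen, blur and respawn logic is disconnected.
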(event `self.ReceiveBeginPlay`
  (bind _returnvalue (`GameplayStatics.GetActorOfClass` "/Game/VRTemplate/Blueprints/VRPawn.VRPawn_C"))
  (set `self.PlayerRef` _returnvalue)
  (bind _outactors (`GameplayStatics.GetAllActorsOfClass` "/Game/zVRContent/blueprints/BP_MapChunk.BP_MapChunk_C"))
  ;[0.3647 0 1] Assign mesh to map chunks
  (`BlueprintMapLibrary.Map_Clear` (`self.MapChunkMeshes`))
  (for _array_element _outactors
    (bind _mesh (`/Game/zVRContent/blueprints/BP_MapChunk.mesh` _array_element))
    (bind _staticmesh (`StaticMeshComponent.StaticMesh` _mesh))
    (set `/Game/zVRContent/blueprints/BP_MapChunk.StaticMesh` _staticmesh _array_element)
    (`SceneComponent.SetVisibility` _mesh false false)
    (bind _returnvalue_2 (`GeometryScriptLibrary_StaticMeshFunctions.CopyMeshFromStaticMesh` _staticmesh (`/Game/zVRContent/blueprints/BP_MapChunk.DynamicMesh` _array_element) (struct) (struct) null)
      (:`Success`
        (`BlueprintMapLibrary.Map_Add` (`self.MapChunkMeshes`) _returnvalue_2 _staticmesh)
        (`GeometryScriptLibrary_MeshSubdivideFunctions.ApplyPNTessellation` _returnvalue_2 (struct) 3 null)
        (`DynamicMeshComponent.SetComplexAsSimpleCollisionEnabled` (`DynamicMeshActor.GetDynamicMeshComponent` _array_element) true true))))
  (set `self.MapChunks` _outactors)
  (`self.EnableInput` (`GameplayStatics.GetPlayerController` 0))
  (bind _returnvalue_3 (`GameplayStatics.GetActorOfClass` "/Game/zVRContent/blueprints/BP_Tree.BP_Tree_C"))
  (`KismetArrayLibrary.Array_Add` (`self.OxygenObjects`) (`/Game/zVRContent/blueprints/BP_Tree.Oxygen` _returnvalue_3))
  ;[0.174 0.4115 0.1136] Post Process Material with decreasing oxygen level
  (bind _returnvalue_4 (`KismetMaterialLibrary.CreateDynamicMaterialInstance` "/Game/zVRContent/materials/Oxygen/M_PP_RadialBlur.M_PP_RadialBlur"))
  (bind _output_get (set `self.DynamicMaterial` _returnvalue_4))
  (set `CameraComponent.PostProcessSettings` (make `PostProcessSettings` :`WeightedBlendables` (make `WeightedBlendables` (`|MakeArray` (make `WeightedBlendable` 1.0 (`self.DynamicMaterial`))))) (`/Game/VRTemplate/Blueprints/VRPawn.Camera` (`self.PlayerRef`)))
  (`MaterialInstanceDynamic.SetScalarParameterValue` _output_get "Blur" 0.0)
  (`MaterialInstanceDynamic.SetScalarParameterValue` _output_get "Blur Radius" 1.0)
  (`MaterialInstanceDynamic.SetScalarParameterValue` _output_get "Blur Radius" 4.0))

(event `EnhancedInput|/Game/VRTemplate/Input/Actions/IA_KeyBoard_P`
  (params (ActionValue :type Boolean) (ElapsedSeconds :type "Float (double-precision)") (TriggeredSeconds :type "Float (double-precision)") (InputAction :type "InputAction Object Reference" :default "/Game/VRTemplate/Input/Actions/IA_KeyBoard_P.IA_KeyBoard_P"))
  (:`Completed`
    (`self.WorldManaging`)))

(event `self.ReceiveTick`
  (params (DeltaSeconds :type "Float (single-precision)"))
  (bind _playerref (`self.PlayerRef`))
  ;[0.3647 0 1] Oxygen
  (for _array_element (`self.OxygenObjects`)
    (bind _output_get (set `/Game/VRTemplate/Blueprints/VRPawn.IsOverlapped` (`PrimitiveComponent.IsOverlappingActor` _array_element _playerref) _playerref))
    (if _output_get
      (break))))

(fn `UserConstructionScript`)

(fn `WorldManaging`
  (bind _treestoupdate (`self.TreesToUpdate`))
  (`|ExecutionSequence`
    (:`then_0`
      ;[0.3647 0 1] Repair Holes
      (for _array_element (`self.MapChunks`)
        (bind _returnvalue (`BaseDynamicMeshComponent.GetDynamicMesh` (`DynamicMeshActor.DynamicMeshComponent` _array_element)))
        (bind (_value _returnvalue_2) (`BlueprintMapLibrary.Map_Find` (`self.MapChunkMeshes`) _returnvalue))
        (if _returnvalue_2
          (`GeometryScriptLibrary_StaticMeshFunctions.CopyMeshFromStaticMesh` _value _returnvalue (struct) (make `GeometryScriptMeshReadLOD` "MaxAvailable") null))))
    (:`then_1`
      ;[0.3647 0 1] Grow trees and remove it from the list when currentState == 3
      (if (not (`KismetArrayLibrary.Array_IsEmpty` _treestoupdate))
        (for _array_element_2 _treestoupdate
          (`|ExecutionSequence`
            (:`then_0`
              (bind _currentstate (`/Game/zVRContent/blueprints/BP_Tree.CurrentState` _array_element_2))
              (if (< _currentstate 3)
                (bind _returnvalue_3 (+ _currentstate 1))
                (`StaticMeshComponent.SetStaticMesh` (`/Game/zVRContent/blueprints/BP_Tree.TreeMesh` _array_element_2) (`BlueprintMapLibrary.Map_Find` (`/Game/zVRContent/blueprints/BP_Tree.TreeStates` _array_element_2) _returnvalue_3))
                (set `/Game/zVRContent/blueprints/BP_Tree.CurrentState` _returnvalue_3 _array_element_2)
                (else
                  (`KismetArrayLibrary.Array_RemoveItem` (`self.TreesToUpdate`) _array_element_2))))
            (:`then_1`
              (if (== _currentstate 1)
                (`SceneComponent.SetRelativeScale3D` (`/Game/zVRContent/blueprints/BP_Tree.Oxygen` _array_element_2) (10.0 10.0 10.0))))))))))